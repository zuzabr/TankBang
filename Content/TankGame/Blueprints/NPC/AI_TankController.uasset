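; AI controller for NPC tanks that runs the BT_Tank behavior tree on possession and feeds its Blackboard.
; On possess it caches the BP_Main_NPC pawn, enables input, then copies movement, bomb-placing and tank type from the NPC's data table row into Blackboard keys.
; Separate update functions write player sighting, bullet sighting and nearby bomb state with location to the Blackboard.
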(event `self.ReceivePossess`
  (params (PossessedPawn :type "Pawn Object Reference"))
  (`self.Init`)
  (`self.RunBehaviorTree` "/Game/TankGame/Blueprints/NPC/BT_Tank.BT_Tank")
  (`self.SetValuesInBB`)
  (`self.CheckForNPCAbilities`))

(fn `CheckForNPCAbilities`
  (bind (_datatable _rowname) (break `DataTableRowHandle` (`.Description_2_838EBF994D755D2F64E9E5BCF961BF3C` (break `/Game/TankGame/Blueprints/Core/ST_TankSpecification` (`/Game/TankGame/Blueprints/Core/BP_Tank.Specification` (`self.NPC`))))))
  (bind _returnvalue (`|GetDataTableRow` _datatable _rowname)
    (:`then`
      (bind (_tanktype _canmove _canplacebombs) (break `/Game/TankGame/Blueprints/Core/S_Tank` _returnvalue))
      (`BlackboardComponent.SetValueAsBool` (`self.Blackboard`) "CanMove" _canmove)
      (`BlackboardComponent.SetValueAsBool` (`self.Blackboard`) "CanPlaceBombs" _canplacebombs)
      (`BlackboardComponent.SetValueAsEnum` (`self.Blackboard`) "TankType" _tanktype))))

(fn `Init`
  (bind _asbp_main_npc (cast `/Game/TankGame/Blueprints/NPC/BP_Main_NPC` (`self.K2_GetPawn`)))
  (set `self.NPC` _asbp_main_npc))

(fn `SetValuesInBB`
  (`BlackboardComponent.SetValueAsBool` (`self.Blackboard`) "InputEnabled" true)
  (`BlackboardComponent.SetValueAsObject` (`self.Blackboard`) "SelfActor" (`self.NPC`)))

(fn `UpdateBB Bomb`
  (params (BombInRadius :type Boolean) (BombLocation :type "Vector Structure"))
  (`BlackboardComponent.SetValueAsBool` (`self.Blackboard`) "NearTheBomb" BombInRadius)
  (`BlackboardComponent.SetValueAsVector` (`self.Blackboard`) "BombLocation" BombLocation))

(fn `UpdateBPBullet`
  (params (BulletSet :type Boolean))
  (`BlackboardComponent.SetValueAsBool` (`self.Blackboard`) "SeeBullet" BulletSet))

(fn `UpdateBPPlayer`
  (params (PlayerSet :type Boolean))
  (`BlackboardComponent.SetValueAsBool` (`self.Blackboard`) "SeePlayer" PlayerSet))

(fn `UserConstructionScript`)