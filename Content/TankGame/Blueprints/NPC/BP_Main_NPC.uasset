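; Base Blueprint for enemy tank NPCs that idly sweep their turret, then track and shoot the player on sight.
; AI Perception pauses or resumes a looping timer that rotates the turret toward the player and updates the AI_TankController.
; Each tick of that timer rolls a random chance to fire, shooting only if TankComponent's trace hits the player.
; Death hides the tank, disables collision, plays effects, then reports its type and color before destroying it.
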(event `NPCDeath`
  ;[1 0 0.2021] Смерть НПС
  (`self.StopLooking`)
  (`KismetSystemLibrary.K2_ClearAndInvalidateTimerHandle` (`self.PlayerFoundTimer`))
  (`self.DisableInput` null)
  (`SceneComponent.SetHiddenInGame` (`self.Mesh`) true true)
  (`PrimitiveComponent.SetCollisionEnabled` (`self.Turret`) "NoCollision")
  (`PrimitiveComponent.SetCollisionEnabled` (`self.Base`) "NoCollision")
  (`PrimitiveComponent.SetCollisionEnabled` (`self.Mesh`) "NoCollision")
  (`PrimitiveComponent.SetCollisionEnabled` (`self.CapsuleComponent`) "NoCollision")
  (`AddComponent|NODE_AddNiagaraComponent-0`)
  (`GameplayStatics.PlaySoundAtLocation` "/Game/TankGame/Music/TankExplosion.TankExplosion" (`self.K2_GetActorLocation`) (struct) 1.0 1.0 0.0 null null self null)
  (`KismetSystemLibrary.Delay` 2.0)
  (`self.DeathNPC`))

(event `self.ReceiveBeginPlay`
  ;[1 1 1] Хаотичное вращение башней для стоячих танков, чтобы не стояли столбом
  (`parent.ReceiveBeginPlay`)
  (`self.GetNPCController`)
  (`self.LookForPlayer`)
  (bind _returnvalue (`KismetSystemLibrary.K2_SetTimer` null "RotationToPlayer" 0.01 true))
  (bind _output_get (set `self.PlayerFoundTimer` _returnvalue))
  (`KismetSystemLibrary.K2_PauseTimerHandle` _output_get)
  (`KismetSystemLibrary.Delay` 1.0)
  (`AIPerceptionComponent.SetSenseEnabled` (`self.AIPerception`) "/Script/AIModule.AISense_Sight" true))

(event `LookForPlayer`
  ;[1 1 1] Хаотичное вращение башней для стоячих танков, чтобы не стояли столбом
  (bind (_direction _rotator) (`Timeline|TurretRotator` :!label _label)
    (:`Update`
      (`SceneComponent.K2_AddLocalRotation` (`self.Turret`) (`KismetMathLibrary.MakeRotator` 0.0 0.0 (* _rotator (`self.RotationSpeed`))) false false))
    (:`Finished`
      (`KismetSystemLibrary.Delay` 0.2)
      (goto _label :!via `Reverse`))))

(event `StopLooking`
  ;[1 1 1] Хаотичное вращение башней для стоячих танков, чтобы не стояли столбом
  (goto _label :!via `Stop`))

(event `self.AIPerception.OnTargetPerceptionUpdated`
  (params (Actor :type "Actor Object Reference") (Stimulus :type "AIStimulus Structure"))
  ;[1 1 1] Стрельба по игроку
  (set `self.Stimulus` Stimulus)
  (bind _asbp_player (cast `/Game/TankGame/Blueprints/Player/BP_Player` Actor)
    (:`then`
      (if (`.bSuccessfullySensed` (break `AIStimulus` (`self.Stimulus`)))
        (`/Engine/EditorBlueprintResources/StandardMacros.IsValid` (`self.NPCController`)
          (:`Is Valid`
            (set `self.PlayerTank` _asbp_player)
            (bind _output_get (set `self.SeeTank` (`.bSuccessfullySensed` (break `AIStimulus` (`self.Stimulus`)))))
            (`/Game/TankGame/Blueprints/NPC/AI_TankController.UpdateBPPlayer` (`self.NPCController`) _output_get)
            (`self.StopLooking`)
            (`KismetSystemLibrary.K2_UnPauseTimerHandle` (`self.PlayerFoundTimer`))))
        (else
          (`/Engine/EditorBlueprintResources/StandardMacros.IsValid` (`self.NPCController`) :!label _label_2
            (:`Is Valid`
              (set `self.SeeTank` false)
              (`/Game/TankGame/Blueprints/NPC/AI_TankController.UpdateBPPlayer` (`self.NPCController`) false)
              (`self.LookForPlayer`)
              (`KismetSystemLibrary.K2_PauseTimerHandle` (`self.PlayerFoundTimer`)))))))
    (:`CastFailed`
      (goto _label_2))))

(fn `Automatic Shoot`
  (if (> (`/Game/TankGame/Blueprints/Core/Tank_Component.Shoot Delta` (`self.Tank_Component`)) (`KismetMathLibrary.RandomFloatInRange` 0.0 100.0))
    (`/Engine/EditorBlueprintResources/StandardMacros.IsValid` (`self.PlayerTank`)
      (:`Is Valid`
        (bind (_lazerend _hitactor) (`/Game/TankGame/Blueprints/Core/Tank_Component.FirstTrace` (`self.Tank_Component`)))
        (if (== _hitactor (`self.PlayerTank`))
          (`/Game/TankGame/Blueprints/Core/Tank_Component.Shoot` (`self.Tank_Component`)))))))

(fn `DeathNPC`
  (`self.NPCDead` (`/Game/TankGame/Blueprints/Core/Tank_Component.Tank Type` (`self.Tank_Component`)) (`/Game/TankGame/Blueprints/Core/Tank_Component.TankColor` (`self.Tank_Component`)))
  (`self.K2_DestroyActor`))

(fn `GetNPCController`
  (bind _asai_tank_controller (cast `/Game/TankGame/Blueprints/NPC/AI_TankController` (`self.GetController`)))
  (set `self.NPCController` _asai_tank_controller))

(fn `RotationToPlayer`
  (bind _playertank (`self.PlayerTank`))
  (bind (_returnvalue_roll _returnvalue_pitch _returnvalue_yaw) (`KismetMathLibrary.BreakRotator` (`KismetMathLibrary.FindLookAtRotation` (`SceneComponent.K2_GetComponentLocation` (`self.Turret`)) (`self.K2_GetActorLocation` _playertank))))
  (`/Engine/EditorBlueprintResources/StandardMacros.IsValid` _playertank
    (:`Is Valid`
      (`self.SetTurretRotation` (`KismetMathLibrary.MakeRotator` 0.0 0.0 _returnvalue_yaw))
      (`self.Automatic Shoot`))))

(fn `SetTurretRotation`
  (params (TargetRotation :type "Rotator Structure"))
  (`SceneComponent.K2_SetWorldRotation` (`self.Turret`) (`KismetMathLibrary.RInterpTo` (`SceneComponent.K2_GetComponentRotation` (`self.Turret`)) TargetRotation (`GameplayStatics.GetWorldDeltaSeconds`) (`self.TurretRotationSpeed`)) false false))

(fn `UserConstructionScript`
  (`parent.UserConstructionScript`))