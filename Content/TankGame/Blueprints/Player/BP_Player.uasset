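; Player tank character that moves, aims, shoots, places bombs and pauses, delegating weapons and laser tracing to TankComponent.
; GM_Tanks' JoyStickIndex selects either axis movement with touch-to-aim-and-fire, or dead-zoned gyroscope movement with joystick turret aiming and button fire.
; Tick updates the laser beam and engine audio parameter, while the game mode setting toggles the light.
; DeathTank spends lives on bullet hits; final or non-bullet death hides the tank and ends the session through GM_Tanks.
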(event `InputAction|Shoot`
  (params (Key :type "Key Structure"))
  ;[0 1 0.2806] Выстрел
  (:`Pressed`
    (if (`self.TurretRotatesViaJoyStick`)
      (`/Game/TankGame/Blueprints/Core/Tank_Component.Shoot` (`self.Tank_Component`)))))

(event `/Game/TankGame/Blueprints/Core/BPI_Tank.RestartAfterLose`
  ;[0.02183 0 1] Рестарт уровня после проигрыша
  (set `self.CurNumberOfLifes` 2)
  (`self.EnableInput` (`GameplayStatics.GetPlayerController` 0))
  (`SceneComponent.SetHiddenInGame` (`self.Mesh`) false true)
  (`SceneComponent.SetHiddenInGame` (`self.Arrow1`) true false))

(event `InputAxis|Rotation(Mouse)`
  (params (AxisValue :type "Float (single-precision)"))
  ;[1 0 0] Вращение башней мышкой (тестирование, убрать)
  (`SceneComponent.K2_AddLocalRotation` (`self.Turret`) (`KismetMathLibrary.MakeRotator` 0.0 0.0 (* AxisValue 2.0)) false false))

(event `self.ReceiveBeginPlay`
  ;[0 1 0.2102] Запись количества жизней и включения света
  (`parent.ReceiveBeginPlay`)
  (set `self.InitNumOfLifes` (`self.CurNumberOfLifes`))
  (bind _asgm_tanks (cast `/Game/TankGame/Blueprints/Core/GM_Tanks` (`GameplayStatics.GetGameMode`)))
  (`self.ChangeMovementInput` (`/Game/TankGame/Blueprints/Core/GM_Tanks.JoyStickIndex` _asgm_tanks))
  (if (`|EnumEquality` (`/Game/TankGame/Blueprints/Core/GM_Tanks.GetCurGMInfo` _asgm_tanks) "NewEnumerator1")
    (`LightComponent.SetIntensity` (`self.Light`) 8000.0)
    (else
      (`LightComponent.SetIntensity` (`self.Light`) 0.0))))

(event `InputAction|PlaceBomb`
  (params (Key :type "Key Structure"))
  ;[0 1 0.2795] Постановка бомбы
  (:`Pressed`
    (`/Game/TankGame/Blueprints/Core/Tank_Component.PlaceBomb` (`self.Tank_Component`))))

(event `PlayerDeath`
  ;[0 0.04148 1] Смерть Игрока
  (`AddComponent|NODE_AddNiagaraComponent-0`)
  (`GameplayStatics.PlaySoundAtLocation` "/Game/TankGame/Music/TankExplosion.TankExplosion" (`self.K2_GetActorLocation`) (struct) 1.0 1.0 0.0 null null self)
  (`KismetSystemLibrary.Delay` 2.0)
  (bind _asgm_tanks (cast `/Game/TankGame/Blueprints/Core/GM_Tanks` (`GameplayStatics.GetGameMode`)))
  (`/Game/TankGame/Blueprints/Core/GM_Tanks.GameSessionEnd` _asgm_tanks false))

(event `InputAction|Pause`
  (params (Key :type "Key Structure"))
  ;[0 1 0.3042] Открывает меню паузы
  (:`Pressed`
    (`GameplayStatics.SetGamePaused` true)
    (bind _asgm_tanks (cast `/Game/TankGame/Blueprints/Core/GM_Tanks` (`GameplayStatics.GetGameMode`)))
    (`/Game/TankGame/Blueprints/Core/GM_Tanks.OpenPauseWidget` _asgm_tanks)))

(event `InputAxis|MoveForward`
  (params (AxisValue :type "Float (single-precision)"))
  ;[1 0.3719 0] Управление мышкой / стиком (надо включить orientation to movement)
  (if (not (`self.GyroMovement`))
    (`self.AddMovementInput` (`KismetMathLibrary.GetForwardVector` (`KismetMathLibrary.MakeRotator` 0.0 0.0 (.yaw (`self.GetControlRotation`)))) AxisValue)))

(event `InputAxis|MoveRight`
  (params (AxisValue :type "Float (single-precision)"))
  ;[1 0.3719 0] Управление мышкой / стиком (надо включить orientation to movement)
  (if (not (`self.GyroMovement`))
    (`self.AddMovementInput` (`KismetMathLibrary.GetRightVector` (`KismetMathLibrary.MakeRotator` 0.0 0.0 (.yaw (`self.GetControlRotation`)))) AxisValue)))

(event `self.ReceiveTick`
  (params (DeltaSeconds :type "Float (single-precision)"))
  ;[1 0 0.6603] Вращение башней на джойстике (подключить)
  (`self.TrackAudio`)
  (`self.LaserSpawn&Update`)
  (if (`self.TurretRotatesViaJoyStick`)
    (`self.TurretRotationViaJoystick` DeltaSeconds)))

(event `InputVectorAxis|Gravity`
  (params (AxisValue :type "Vector Structure"))
  ;[1 0 0.5732] Управление танком с помощью гироскопа (надо выключить orientation to movement)
  (if (`self.GyroMovement`)
    (`self.ForwardMove` AxisValue_X)
    (`self.RightMove` AxisValue_Y)
    (`self.GyroscopeMovement`)))

(event `InputTouch`
  (params (Location :type "Vector Structure") (FingerIndex :type "ETouchIndex Enum"))
  ;[1 0.3276 0] Выстрел и поворот башни касанием
  (:`Pressed`
    (if (not (`self.TurretRotatesViaJoyStick`))
      (`self.TurretRotationViaFinger` FingerIndex)
      (`/Game/TankGame/Blueprints/Core/Tank_Component.Shoot` (`self.Tank_Component`))))
  (:`Moved`
    (if (not (`self.TurretRotatesViaJoyStick`))
      (`self.TurretRotationViaFinger` FingerIndex))))

(fn `ChangeMovementInput`
  (params (JoyStickIndex :type Integer))
  (if (< JoyStickIndex 2)
    (set `CharacterMovementComponent.bOrientRotationToMovement` true (`self.CharacterMovement`))
    (set `self.TurretRotatesViaJoyStick` false)
    (set `self.GyroMovement` false)
    (else
      (set `CharacterMovementComponent.bOrientRotationToMovement` false (`self.CharacterMovement`))
      (set `self.TurretRotatesViaJoyStick` true)
      (set `self.GyroMovement` true))))

(fn `DeathTank`
  (params (ByBullet :type Boolean))
  (if ByBullet
    (if (> (`self.CurNumberOfLifes`) 0)
      (`/Engine/EditorBlueprintResources/StandardMacros.DecrementInt` (`self.CurNumberOfLifes`))
      (else
        (set `self.CurNumberOfLifes` -1 :!label _label)
        (`self.DisableInput` (`GameplayStatics.GetPlayerController` 0))
        (`SceneComponent.SetHiddenInGame` (`self.Mesh`) true true)
        (`self.PlayerDeath`)))
    (else
      (goto _label))))

(fn `ForwardMove`
  (params (AxisValue :type "Float (double-precision)"))
  (locals (L_AxisValue :type "Float (double-precision)"))
  ;[1 1 1] Обект начинает двигать при значении больше 1 и меньше -1 (цифра может варьироваться)
  (set `local.L_AxisValue` (* AxisValue -1.0))
  (if (> (`local.L_AxisValue`) 0.2)
    (set `self.AxisValueForward` (`local.L_AxisValue`))
    (elif (< (`local.L_AxisValue`) (* 2.0 -1.0))
      (set `self.AxisValueForward` (`local.L_AxisValue`))
      (else
        (set `self.AxisValueForward` 0.0)))))

(fn `GyroscopeMovement`
  (bind _returnvalue (* (`KismetMathLibrary.ClampVectorSize` (`KismetMathLibrary.MakeVector` (`self.AxisValueForward`) (`self.AxisValueRight`)) 0.0 1.0) (* (`GameplayStatics.GetWorldDeltaSeconds`) 300.0)))
  (bind _returnvalue_2 (`KismetMathLibrary.VSize` _returnvalue))
  (if (> _returnvalue_2 0.0)
    (`SceneComponent.K2_SetWorldRotation` (`self.CapsuleComponent`) (`KismetMathLibrary.RInterpTo` (`SceneComponent.K2_GetComponentRotation` (`self.CapsuleComponent`)) (`KismetMathLibrary.Conv_VectorToRotator` _returnvalue) (`GameplayStatics.GetWorldDeltaSeconds`) 5.0) false false)
    (`self.AddMovementInput` _returnvalue _returnvalue_2)))

(fn `LaserSpawn&Update`
  (bind _laser (`self.Laser`))
  (`ParticleSystemComponent.SetBeamSourcePoint` _laser 0 (`SceneComponent.K2_GetComponentLocation` (`self.Arrow1`)) 0)
  (bind _lazerend (`/Game/TankGame/Blueprints/Core/Tank_Component.FirstTracePlayer` (`self.Tank_Component`)))
  (`ParticleSystemComponent.SetBeamTargetPoint` _laser 0 _lazerend 0))

(fn `RightMove`
  (params (AxisValue :type "Float (double-precision)"))
  (locals (L_AxisValue :type "Float (double-precision)"))
  ;[1 1 1] Обект начинает двигать при значении больше 1 и меньше -1 (цифра может варьироваться)
  (set `local.L_AxisValue` AxisValue)
  (if (> (`local.L_AxisValue`) (`self.GyroscopeSensitivity`))
    (set `self.AxisValueRight` (`local.L_AxisValue`))
    (elif (< (`local.L_AxisValue`) (* (`self.GyroscopeSensitivity`) -1.0))
      (set `self.AxisValueRight` (`local.L_AxisValue`))
      (else
        (set `self.AxisValueRight` 0.0)))))

(fn `SetTurretInitialRotation`
  ;[1 1 1] Сохранение изначального положения турели
  (`SceneComponent.K2_SetRelativeRotation` (`self.Turret`) (`KismetMathLibrary.RInterpTo` (`SceneComponent.RelativeRotation` (`self.Turret`)) (`self.InitialRotation`) 0.5 0.05) false false))

(fn `TrackAudio`
  (if (!= (`self.GetVelocity`) (0.0 0.0 0.0))
    (`AudioComponent.SetFloatParameter` (`self.Audio`) "TankSpeed" 10.0)
    (else
      (`AudioComponent.SetFloatParameter` (`self.Audio`) "TankSpeed" 300.0))))

(fn `TurretRotationViaFinger`
  (params (FingerIndex :type "ETouchIndex Enum" :default "Touch1"))
  (bind (_returnvalue_roll _returnvalue_pitch _returnvalue_yaw) (`KismetMathLibrary.BreakRotator` (`KismetMathLibrary.FindLookAtRotation` (`SceneComponent.K2_GetComponentLocation` (`self.CapsuleComponent`)) (`.Location` (`GameplayStatics.BreakHitResult` (`PlayerController.GetHitResultUnderFingerByChannel` (`GameplayStatics.GetPlayerController` 0) FingerIndex "TraceTypeQuery1" true))))))
  (`SceneComponent.K2_SetWorldRotation` (`self.Turret`) (`KismetMathLibrary.RInterpTo` (`SceneComponent.K2_GetComponentRotation` (`self.Turret`)) (`KismetMathLibrary.MakeRotator` 0.0 0.0 _returnvalue_yaw) (`GameplayStatics.GetWorldDeltaSeconds`)) true false))

(fn `TurretRotationViaJoystick`
  (params (DeltaSeconds :type "Float (double-precision)"))
  (bind _returnvalue (* (`KismetMathLibrary.ClampVectorSize` (`KismetMathLibrary.MakeVector` (`self.GetInputAxisValue`) (`self.GetInputAxisValue`)) 0.0 1.0) (* DeltaSeconds (`self.MovementSpeed`))))
  ;[1 1 1] Ручное управление турелью
  (if (> (`KismetMathLibrary.VSize` _returnvalue) 0.0)
    (`SceneComponent.K2_SetWorldRotation` (`self.Turret`) (`KismetMathLibrary.Conv_VectorToRotator` _returnvalue) false false)))

(fn `UserConstructionScript`
  (`parent.UserConstructionScript`)
  (`ActorComponent.SetAutoActivate` (`self.AIPerceptionStimuliSource`) true))