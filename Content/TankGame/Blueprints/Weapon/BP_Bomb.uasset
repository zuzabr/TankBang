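; Timed bomb owned by a tank that switches to a blinking material shortly before exploding.
; Explosion sends hit or explode messages to tanks, weapons and cubes overlapping its radius, crediting the owning tank for tank hits.
; Another bomb's blast triggers it early via BombInterexplosion, which relays only to BP_BulletDefault among weapons.
; DestroyBomb fires BombDestroyed, hides the bomb and plays effects before delayed destruction, while RestartAfterLose removes it without exploding.
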(event `self.ReceiveBeginPlay`
  (bind _timerforbomb (`self.TimerForBomb`))
  (bind _asbp_tank (cast `/Game/TankGame/Blueprints/Core/BP_Tank` (`self.GetOwner`)))
  (set `self.OwnerTank` _asbp_tank)
  (bind _returnvalue (`KismetSystemLibrary.K2_SetTimerDelegate` (delegate `InitiateExplosion`) _timerforbomb))
  (set `self.Timer` _returnvalue)
  (`KismetSystemLibrary.Delay` (- _timerforbomb 2.0))
  (`PrimitiveComponent.SetMaterial` (`self.Bomb`) 0 "/Game/TankGame/Materials/M_Blinker.M_Blinker"))

(event `InitiateExplosion`
  (if (not (`SceneComponent.bHiddenInGame` (`self.Bomb`)))
    (`self.Explosion`)))

(event `/Game/TankGame/Blueprints/Weapon/BPI_Weapon.BombExplode`
  (params (Bomb :type "/Game/TankGame/Blueprints/Weapon/BP_Bomb Object Reference"))
  (`self.BombInterexplosion` Bomb))

(event `/Game/TankGame/Blueprints/Weapon/BPI_Weapon.RestartAfterLose`
  (if (`KismetSystemLibrary.K2_TimerExistsHandle` (`self.Timer`))
    (`KismetSystemLibrary.K2_ClearAndInvalidateTimerHandle` (`self.Timer`)))
  (`self.BombDestroyed_0`)
  (`self.K2_DestroyActor`))

(event `BombBlust`
  (`/Engine/EditorBlueprintResources/StandardMacros.DoOnce` false
    (:`Completed`
      (`AddComponent|NODE_AddNiagaraComponent-2`)
      (`GameplayStatics.PlaySoundAtLocation` "/Game/TankGame/Music/BombExplosion.BombExplosion" (`self.K2_GetActorLocation`) (struct) 1.0 1.0 0.0 null null self)
      (`KismetSystemLibrary.Delay` 2.0)
      (`self.K2_DestroyActor`))))

(fn `BombInterexplosion`
  (params (Bomb :type "/Game/TankGame/Blueprints/Weapon/BP_Bomb Object Reference"))
  (bind _explosionradius (`self.ExplosionRadius`))
  (if (!= Bomb self)
    (`KismetSystemLibrary.K2_ClearAndInvalidateTimerHandle` (`self.Timer`))
    (`|ExecutionSequence`
      (:`then_0`
        (for _array_element (`PrimitiveComponent.GetOverlappingActors` _explosionradius "/Game/TankGame/Blueprints/Core/BP_Tank.BP_Tank_C")
          (message `/Game/TankGame/Blueprints/Core/BPI_Tank.HitByBomb` _array_element (`self.OwnerTank`))))
      (:`then_1`
        (for _array_element_2 (`PrimitiveComponent.GetOverlappingActors` _explosionradius "/Game/TankGame/Blueprints/Weapon/BP_Weapon.BP_Weapon_C")
          (bind _asbp_bullet_default (cast `/Game/TankGame/Blueprints/Weapon/BP_BulletDefault` _array_element_2))
          (message `/Game/TankGame/Blueprints/Weapon/BPI_Weapon.BombExplode` _asbp_bullet_default self)))
      (:`then_2`
        (for _array_element_3 (`PrimitiveComponent.GetOverlappingActors` _explosionradius "/Game/TankGame/Blueprints/InteractiveObjects/BP_Cube.BP_Cube_C")
          (message `/Game/TankGame/Blueprints/Weapon/BPI_Weapon.BombExplode` _array_element_3 self)))
      (:`then_3`
        (`self.DestroyBomb`)))))

(fn `DestroyBomb`
  (if (`KismetSystemLibrary.K2_TimerExistsHandle` (`self.Timer`))
    (`KismetSystemLibrary.K2_ClearAndInvalidateTimerHandle` (`self.Timer`)))
  (`self.BombDestroyed_0`)
  (`SceneComponent.SetHiddenInGame` (`self.Bomb`) true false)
  (`PrimitiveComponent.SetCollisionEnabled` (`self.Bomb`) "NoCollision")
  (`PrimitiveComponent.SetCollisionEnabled` (`self.SphereCollision`) "NoCollision")
  (`PrimitiveComponent.SetCollisionEnabled` (`self.ExplosionRadius`) "NoCollision")
  (`self.BombBlust`))

(fn `Explosion`
  (bind _explosionradius (`self.ExplosionRadius`))
  (`KismetSystemLibrary.K2_ClearAndInvalidateTimerHandle` (`self.Timer`))
  (`|ExecutionSequence`
    (:`then_0`
      (for _array_element (`PrimitiveComponent.GetOverlappingActors` _explosionradius "/Game/TankGame/Blueprints/Core/BP_Tank.BP_Tank_C")
        (message `/Game/TankGame/Blueprints/Core/BPI_Tank.HitByBomb` _array_element (`self.OwnerTank`))))
    (:`then_1`
      (for _array_element_2 (`PrimitiveComponent.GetOverlappingActors` _explosionradius "/Game/TankGame/Blueprints/Weapon/BP_Weapon.BP_Weapon_C")
        (message `/Game/TankGame/Blueprints/Weapon/BPI_Weapon.BombExplode` _array_element_2 self)))
    (:`then_2`
      (for _array_element_3 (`PrimitiveComponent.GetOverlappingActors` _explosionradius "/Game/TankGame/Blueprints/InteractiveObjects/BP_Cube.BP_Cube_C")
        (message `/Game/TankGame/Blueprints/Weapon/BPI_Weapon.BombExplode` _array_element_3 self)))
    (:`then_3`
      (`self.DestroyBomb`))))

(fn `UserConstructionScript`
  (`parent.UserConstructionScript`))