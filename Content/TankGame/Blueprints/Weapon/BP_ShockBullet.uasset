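; BP_ShockBullet is a bullet variant for the tank game that delivers a shock hit to tanks.
; On hit it tests bullet, tank and bomb in turn, falling back to a miss handler; all but the tank check defer to the parent.
; The tank override sends a shock message, or a regular bullet hit with owner and tank type if ShockWorks is already set, then destroys the bullet.
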(event `self.ReceiveHit`
  (params (MyComp :type "PrimitiveComponent Object Reference") (Other :type "Actor Object Reference") (OtherComp :type "PrimitiveComponent Object Reference") (bSelfMoved :type Boolean) (HitLocation :type "Vector Structure") (HitNormal :type "Vector Structure") (NormalImpulse :type "Vector Structure") (Hit :type "HitResult Structure (by ref)"))
  (bind (_bblockinghit _binitialoverlap _time _distance _location _impactpoint _normal _impactnormal _physmat _hitactor _hitcomponent) (`GameplayStatics.BreakHitResult` Hit))
  (bind _hitsmth (`self.BulletHitBullet` _hitactor))
  (if (not _hitsmth)
    (bind _hitsmth_2 (`self.BulletHitTank` _hitactor))
    (if (not _hitsmth_2)
      (bind _hitsmth_3 (`self.BulletHitBomb` _hitactor _hitcomponent))
      (if (not _hitsmth_3)
        (`self.BulletHitNothing`)))))

(fn `BulletHitBomb`
  (params (Actor :type "Actor Object Reference") (Component :type "PrimitiveComponent Object Reference"))
  (`parent.BulletHitBomb` Actor Component))

(fn `BulletHitBullet`
  (params (Actor :type "Actor Object Reference"))
  (`parent.BulletHitBullet` Actor))

(fn `BulletHitNothing`
  (`parent.BulletHitNothing`))

(fn `BulletHitTank`
  (params (Actor :type "Actor Object Reference"))
  (if (>= (`self.GetNumberOfHits`) 0)
    (bind _asbp_tank (cast `/Game/TankGame/Blueprints/Core/BP_Tank` Actor))
    (set `self.HitSmth` true)
    (if (`/Game/TankGame/Blueprints/Core/BP_Tank.ShockWorks` _asbp_tank)
      (message `/Game/TankGame/Blueprints/Core/BPI_Tank.HitByBullet` _asbp_tank (`self.TankOwner`) (`self.Tank Type`))
      (else
        (message `/Game/TankGame/Blueprints/Core/BPI_Tank.HitByShockBullet` _asbp_tank)))
    (`self.DestroyBullet`)))

(fn `UserConstructionScript`
  (`parent.UserConstructionScript`))