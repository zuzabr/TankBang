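; BP_BulletDefault is the tank projectile that ricochets a limited number of times and damages what it hits.
; On spawn it reads tank type, ricochet limit and color from the owning tank's data table row, tinting a dynamic material.
; Hits check bullet, bomb, then tank; anything else counts as a ricochet, playing a sound until the limit destroys it.
; Bomb explosion and restart-after-loss events also destroy it.
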(event `self.ReceiveBeginPlay`
  ;[1 1 1] Получает данные
  (bind _asbp_tank (cast `/Game/TankGame/Blueprints/Core/BP_Tank` (`self.GetOwner`)))
  (bind _output_get (set `self.TankOwner` _asbp_tank))
  (bind (_datatable _rowname) (break `DataTableRowHandle` (`.Description_2_838EBF994D755D2F64E9E5BCF961BF3C` (break `/Game/TankGame/Blueprints/Core/ST_TankSpecification` (`/Game/TankGame/Blueprints/Core/BP_Tank.Specification` _output_get)))))
  (bind _returnvalue (`|GetDataTableRow` _datatable _rowname)
    (:`then`
      (bind (_tanktype _canmove _canplacebombs _numberofricochets _numberofbullets _numberofbombs _tankspeed _bullettype _material _color) (break `/Game/TankGame/Blueprints/Core/S_Tank` _returnvalue))
      (set `self.Tank Type` _tanktype)
      (set `self.Number Of Ricochets` _numberofricochets)
      (bind _returnvalue_2 (`PrimitiveComponent.CreateDynamicMaterialInstance` (`self.Bullet`) 0 "/Game/TankGame/Materials/M_Bullet.M_Bullet" "None"))
      (`MaterialInstanceDynamic.SetVectorParameterValue` _returnvalue_2 "BulletColor" _color))))

(event `/Game/TankGame/Blueprints/Weapon/BPI_Weapon.BombExplode`
  (params (Bomb :type "/Game/TankGame/Blueprints/Weapon/BP_Bomb Object Reference"))
  ;[1 1 1] Мгновенное уничтожение пули по различным причинам
  (`self.DestroyBullet`))

(event `/Game/TankGame/Blueprints/Weapon/BPI_Weapon.RestartAfterLose`
  ;[1 1 1] Мгновенное уничтожение пули по различным причинам
  (`self.DestroyBullet`))

(event `self.ReceiveHit`
  (params (MyComp :type "PrimitiveComponent Object Reference") (Other :type "Actor Object Reference") (OtherComp :type "PrimitiveComponent Object Reference") (bSelfMoved :type Boolean) (HitLocation :type "Vector Structure") (HitNormal :type "Vector Structure") (NormalImpulse :type "Vector Structure") (Hit :type "HitResult Structure (by ref)"))
  (bind (_bblockinghit _binitialoverlap _time _distance _location _impactpoint _normal _impactnormal _physmat _hitactor _hitcomponent) (`GameplayStatics.BreakHitResult` Hit))
  ;[1 1 1] Логика попадания пули в различные объекты
  (bind _hitsmth (`self.BulletHitBullet` _hitactor))
  (if (not _hitsmth)
    (bind _hitsmth_2 (`self.BulletHitBomb` _hitactor _hitcomponent))
    (if (not _hitsmth_2)
      (bind _hitsmth_3 (`self.BulletHitTank` _hitactor))
      (if (not _hitsmth_3)
        (`self.BulletHitNothing`)))))

(fn `BulletHitBomb`
  (params (Actor :type "Actor Object Reference") (Component :type "PrimitiveComponent Object Reference"))
  (returns (HitSmth :type Boolean))
  (bind _asbp_bomb (cast `/Game/TankGame/Blueprints/Weapon/BP_Bomb` Actor)
    (:`then`
      (if (== (`/Game/TankGame/Blueprints/Weapon/BP_Bomb.Bomb` _asbp_bomb) Component)
        (set `self.HitSmth` true)
        (`/Game/TankGame/Blueprints/Weapon/BP_Bomb.InitiateExplosion` _asbp_bomb)
        (return true)
        (else
          _)))
    (:`CastFailed`
      _))
  (return false))

(fn `BulletHitBullet`
  (params (Actor :type "Actor Object Reference"))
  (returns (HitSmth :type Boolean))
  (cast `/Game/TankGame/Blueprints/Weapon/BP_BulletDefault` Actor
    (:`then`
      (set `self.HitSmth` true)
      (`self.DestroyBullet`)
      (return true))
    (:`CastFailed`
      (return false))))

(fn `BulletHitNothing`
  (`/Engine/EditorBlueprintResources/StandardMacros.IncrementInt` (`self.NumberOfHits`)
    (:`  `
      (if (> (`self.NumberOfHits`) (`self.Number Of Ricochets`))
        (`self.DestroyBullet`)
        (elif (not (`self.HitSmth`))
          (`GameplayStatics.PlaySoundAtLocation` "/Game/TankGame/Music/Ricochet.Ricochet" (`self.K2_GetActorLocation`) (struct) 1.0 1.0 0.0 null null self))))))

(fn `BulletHitTank`
  (params (Actor :type "Actor Object Reference"))
  (returns (HitSmth :type Boolean))
  (if (>= (`self.NumberOfHits`) 0)
    (bind _asbp_tank (cast `/Game/TankGame/Blueprints/Core/BP_Tank` Actor)
      (:`then`
        (message `/Game/TankGame/Blueprints/Core/BPI_Tank.HitByBullet` _asbp_tank (`self.TankOwner`) (`self.Tank Type`))
        (`self.DestroyBullet`)
        (set `self.HitSmth` true)
        (return true))
      (:`CastFailed`
        _)))
  (return false))

(fn `DestroyBullet`
  (`self.BulletDestroyed`)
  (`self.K2_DestroyActor`))

(fn `GetNumberOfHits`
  (returns (NumberOfHits :type Integer))
  (return (`self.NumberOfHits`)))

(fn `UserConstructionScript`
  (`parent.UserConstructionScript`))