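; BP_Tank is the base tank character shared by BP_Player and BP_Main_NPC, handling setup and hit reactions.
; The construction script reads speed, color and material from a data table row and tints Base and Turret.
; Bullet and bomb hits trace down to place a color-tinted cross decal, register it in GM_Tanks, then route death by subclass cast.
; Shock bullets temporarily cut walk speed and set a shock flag.
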(event `self.ReceiveBeginPlay`
  ;[1 1 1] Рисование следов от танка
  (set `self.InitialSpeed` (`CharacterMovementComponent.MaxWalkSpeed` (`self.CharacterMovement`))))

(event `/Game/TankGame/Blueprints/Core/BPI_Tank.HitByBullet`
  (params (ByWhom :type "/Game/TankGame/Blueprints/Core/BP_Tank Object Reference") (`Tank Type` :type "/Game/TankGame/Blueprints/Core/E_TankTypes Enum" :default "NewEnumerator0"))
  ;[1 1 1] Реакция на попадание пули, дописать логику
  (`self.CrossDrawing`)
  (`self.Death` self true))

(event `/Game/TankGame/Blueprints/Core/BPI_Tank.HitByBomb`
  (params (Owner :type "/Game/TankGame/Blueprints/Core/BP_Tank Object Reference"))
  ;[1 1 1] Реакция на взрыв бомбы
  (`self.CrossDrawing`)
  (`self.Death` self))

(event `/Game/TankGame/Blueprints/Core/BPI_Tank.HitByShockBullet`
  ;[1 1 1] Попадание шоковой пули
  (if (<= (`CharacterMovementComponent.MaxWalkSpeed` (`self.CharacterMovement`)) 5.0)
    (set `self.ShockWorks` true)
    (`KismetSystemLibrary.Delay` 5.0)
    (set `self.ShockWorks` false)
    (else
      (set `CharacterMovementComponent.MaxWalkSpeed` 50.0 (`self.CharacterMovement`))
      (set `self.ShockWorks` true)
      (`KismetSystemLibrary.Delay` 5.0)
      (set `CharacterMovementComponent.MaxWalkSpeed` (`self.InitialSpeed`) (`self.CharacterMovement`))
      (set `self.ShockWorks` false))))

(fn `CrossDrawing`
  (bind _returnvalue (`SceneComponent.K2_GetComponentLocation` (`self.Cross`)))
  (cast `/Game/TankGame/Blueprints/NPC/BP_Main_NPC` self
    (:`then`
      (`/Engine/EditorBlueprintResources/StandardMacros.DoOnce` false
        (:`Completed`
          _)))
    (:`CastFailed`
      _))
  (bind (_outhit _returnvalue_2) (`KismetSystemLibrary.LineTraceSingle` (+ _returnvalue (0.0 0.0 20.0)) (+ _returnvalue (0.0 0.0 -200.0)) "TraceTypeQuery1"))
  (if _returnvalue_2
    (bind _returnvalue_3 (`GameplayStatics.SpawnDecalAtLocation` "/Game/TankGame/Materials/M_Cross.M_Cross" (60.0 60.0 60.0) (`.Location` (`GameplayStatics.BreakHitResult` _outhit))))
    (bind _asgm_tanks (cast `/Game/TankGame/Blueprints/Core/GM_Tanks` (`GameplayStatics.GetGameMode`)))
    (`KismetArrayLibrary.Array_Add` (`/Game/TankGame/Blueprints/Core/GM_Tanks.CrossDecals` _asgm_tanks) _returnvalue_3)
    (bind _returnvalue_4 (`DecalComponent.CreateDynamicMaterialInstance` _returnvalue_3))
    (`MaterialInstanceDynamic.SetVectorParameterValue` _returnvalue_4 "CrossColor" (`self.TankColor`))))

(fn `Death`
  (params (Tank :type "/Game/TankGame/Blueprints/Core/BP_Tank Object Reference") (ByBullet :type Boolean))
  (`KismetSystemLibrary.K2_ClearAndInvalidateTimerHandle` (`self.TimerForCheckingSpeed`))
  (`|ExecutionSequence`
    (:`then_0`
      (bind _asbp_player (cast `/Game/TankGame/Blueprints/Player/BP_Player` Tank))
      (`/Game/TankGame/Blueprints/Player/BP_Player.DeathTank` _asbp_player ByBullet))
    (:`then_1`
      (bind _asbp_main_npc (cast `/Game/TankGame/Blueprints/NPC/BP_Main_NPC` Tank))
      (`/Game/TankGame/Blueprints/NPC/BP_Main_NPC.NPCDeath` _asbp_main_npc))))

(fn `GetTankColor`
  (returns (TankColor :type "LinearColor Structure"))
  (return (`self.TankColor`)))

(fn `UserConstructionScript`
  (bind (_datatable _rowname) (break `DataTableRowHandle` (`.Description_2_838EBF994D755D2F64E9E5BCF961BF3C` (break `/Game/TankGame/Blueprints/Core/ST_TankSpecification` (`self.Specification`)))))
  (bind _returnvalue (`|GetDataTableRow` _datatable _rowname)
    (:`then`
      (`|ExecutionSequence`
        (:`then_0`
          (bind (_tanktype _canmove _canplacebombs _numberofricochets _numberofbullets _numberofbombs _tankspeed _bullettype _material _color) (break `/Game/TankGame/Blueprints/Core/S_Tank` _returnvalue))
          (set `CharacterMovementComponent.MaxWalkSpeed` _tankspeed (`self.CharacterMovement`)))
        (:`then_1`
          (set `self.TankColor` _color))
        (:`then_2`
          ;[1 1 1] установка цвета танка
          (`/Engine/EditorBlueprintResources/StandardMacros.IsValid` _material
            (:`Is Valid`
              (bind _returnvalue_2 (`PrimitiveComponent.CreateDynamicMaterialInstance` (`self.Base`) 0 _material "None"))
              (`MaterialInstanceDynamic.SetVectorParameterValue` _returnvalue_2 "MainColor" _color)
              (bind _returnvalue_3 (`PrimitiveComponent.CreateDynamicMaterialInstance` (`self.Turret`) 0 _material "None"))
              (`MaterialInstanceDynamic.SetVectorParameterValue` _returnvalue_3 "MainColor" _color))))))))