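; Save game object for the tank game, holding player progress and options between sessions.
; It stores full stars collected, level info, last level name, game mode, destroyed NPC tanks and remaining bullets.
; It also keeps music and effects sound, touch interface and joystick index settings.
; Simple setter and getter functions only write or return these variables; no disk saving or loading happens here.
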(fn `Get Settings`
  (returns (MusicSound :type Boolean) (EffectSound :type Boolean) (`Touch Interface` :type "TouchInterface Object Reference") (JoyStickIndex :type Integer))
  (return (`self.MusicSound`) (`self.EffectsSound`) (`self.Touch Interface`) (`self.JoyStickIndex`)))

(fn `GetBulletsRemain`
  (returns (BulletsRemain :type Integer))
  (return (`self.BulletsRemain`)))

(fn `GetGameMode`
  (returns (GameMode :type "DataTableRowHandle Structure"))
  (return (`self.GameMode`)))

(fn `GetLevelName`
  (returns (NewParam :type Name))
  (return (`self.LastLevel`)))

(fn `GetNPCDestroyed`
  (returns (NPCDead :type "Array of /Game/TankGame/Blueprints/Core/ST_NPCDeath Structure"))
  (return (`self.NPCDead`)))

(fn `LoadGame`
  (returns (FullStarsCollected :type Integer) (LevelInfo :type "Array of /Game/TankGame/Widgets/LevelSelection/ST_lvlInfo Structure"))
  (return (`self.FullStarsCollected`) (`self.LevelInfo`)))

(fn `Save Settings`
  (params (MusicSound :type Boolean) (EffectSound :type Boolean) (TouchInterface :type "TouchInterface Object Reference") (JoyStickIndex :type Integer))
  (set `self.MusicSound` MusicSound)
  (set `self.EffectsSound` EffectSound)
  (set `self.Touch Interface` TouchInterface)
  (set `self.JoyStickIndex` JoyStickIndex))

(fn `SaveBulletsRemain`
  (params (NumOfBullets :type Integer))
  (set `self.BulletsRemain` NumOfBullets))

(fn `SaveFullStars`
  (params (FullStarsCollected :type Integer))
  (set `self.FullStarsCollected` FullStarsCollected))

(fn `SaveGameMode`
  (params (GameMode :type "DataTableRowHandle Structure"))
  (set `self.GameMode` GameMode))

(fn `SaveLevelInfo`
  (params (LevelInfo :type "Array of /Game/TankGame/Widgets/LevelSelection/ST_lvlInfo Structure"))
  (set `self.LevelInfo` LevelInfo))

(fn `SaveLevelName`
  (params (LevelName :type Name))
  (set `self.LastLevel` LevelName))

(fn `SaveTanksDestroyed`
  (params (`NPC Dead` :type "Array of /Game/TankGame/Blueprints/Core/ST_NPCDeath Structure"))
  (set `self.NPCDead` `NPC Dead`))