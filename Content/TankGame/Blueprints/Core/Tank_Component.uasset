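; Tank component that handles shooting and bomb placement for BP_Tank owners, both player and NPC.
; On BeginPlay it loads the tank's specification from a DataTable row.
; Bullets and bombs are capped by live counters with destroy-event bindings, except in one game mode where player bullets come from GM_Tanks.
; NPCs fire after a turret line trace or mirrored-vector ricochet sphere traces find a tank, holding fire on other NPCs.
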(event `self.ReceiveBeginPlay`
  (`self.GetOwnerTank`)
  (`self.GetCurrentGM`)
  (`self.SetTankSpecification`))

(fn `ChangeBombCount`
  (set `self.BombCounter` (`KismetMathLibrary.Max` (- (`self.BombCounter`) 1))))

(fn `ChangeBulletCount`
  (set `self.BulletCounter` (`KismetMathLibrary.Max` (- (`self.BulletCounter`) 1))))

(fn `CheckForBombPlacement`
  (returns (CanPlace :type Boolean))
  (if (and (`self.Can Place Bombs`) (< (`self.BombCounter`) (`self.NumberOfBombs`)))
    (return true)
    (else
      (return false))))

(fn `FirstTrace`
  (returns (LazerEnd :type "Vector Structure") (HitActor :type "Actor Object Reference"))
  (bind _turret (`/Game/TankGame/Blueprints/Core/BP_Tank.Turret` (`self.Tank`)))
  (bind _returnvalue (`SceneComponent.K2_GetComponentLocation` _turret))
  (bind _outhit (`KismetSystemLibrary.LineTraceSingle` _returnvalue (+ _returnvalue (* (`SceneComponent.GetForwardVector` _turret) 5000.0)) "TraceTypeQuery1" false (`|MakeArray` (`self.Tank`) :!type "Actor Object Reference") "None" true (struct :`R` 1.0 :`A` 1.0) (struct :`G` 1.0 :`A` 1.0) 2.0))
  (set `self.PreviousHit` _outhit)
  (return (`self.LazerEnd`) (`.HitActor` (`GameplayStatics.BreakHitResult` _outhit))))

(fn `FirstTracePlayer`
  (returns (LazerEnd :type "Vector Structure") (HitActor :type "Actor Object Reference"))
  (bind _turret (`/Game/TankGame/Blueprints/Core/BP_Tank.Turret` (`self.Tank`)))
  (bind _returnvalue (`SceneComponent.K2_GetComponentLocation` _turret))
  (bind _returnvalue_2 (+ _returnvalue (* (`SceneComponent.GetForwardVector` _turret) 5000.0)))
  (bind (_outhit _returnvalue_3) (`KismetSystemLibrary.LineTraceSingle` _returnvalue _returnvalue_2 "TraceTypeQuery1" false (`|MakeArray` (`self.Bullet`) :!type "Actor Object Reference") "None" true (struct :`R` 1.0 :`A` 1.0) (struct :`G` 1.0 :`A` 1.0) 2.0))
  (set `self.PreviousHit` _outhit)
  (if _returnvalue_3
    (bind (_bblockinghit _binitialoverlap _time _distance _location _impactpoint _normal _impactnormal _physmat _hitactor) (`GameplayStatics.BreakHitResult` _outhit))
    (set `self.LazerEnd` _location)
    (else
      (set `self.LazerEnd` _returnvalue_2)))
  (return (`self.LazerEnd`) _hitactor))

(fn `GetBulletCount`
  (returns (BulletCount :type Integer))
  (return (`self.BulletCounter`)))

(fn `GetCurrentGM`
  (bind _asgm_tanks (cast `/Game/TankGame/Blueprints/Core/GM_Tanks` (`GameplayStatics.GetGameMode`)))
  (set `self.GameMode` _asgm_tanks)
  (set `self.CurGame Mode` (`/Game/TankGame/Blueprints/Core/GM_Tanks.GetCurGMInfo` _asgm_tanks)))

(fn `GetLazerCoordinates`
  (returns (LazerEnd :type "Vector Structure"))
  (return (`self.LazerEnd`)))

(fn `GetOwnerTank`
  (bind _asbp_tank (cast `/Game/TankGame/Blueprints/Core/BP_Tank` (`self.GetOwner`)))
  (set `self.Tank` _asbp_tank))

(fn `NPCShoot`
  (bind (_lazerend _hitactor) (`self.FirstTrace`))
  (cast `/Game/TankGame/Blueprints/NPC/BP_Main_NPC` _hitactor
    (:`CastFailed`
      (bind _asbp_player (cast `/Game/TankGame/Blueprints/Player/BP_Player` _hitactor)
        (:`then`
          ;[1 1 1] NPC выстрелит, если нашел игрока попрямой, нпс не стоит на пути пули
          (set `self.TankToHit` _asbp_player)
          (`self.Shoot`))
        (:`CastFailed`
          ;[0.008117 0 1] Если НПС не нашел танк попрямой, проверит на попадание по рикошету и выстрелит, если на пути нет НПС
          (bind (_tankfound _previoushit _tanktohit) (`self.RicochetTraces`))
          (cast `/Game/TankGame/Blueprints/NPC/BP_Main_NPC` _tanktohit
            (:`CastFailed`
              (if _tankfound
                (`self.Shoot`)))))))))

(fn `PlaceBomb`
  (returns (Placed :type Boolean) (BombLocation :type "Vector Structure"))
  (bind _returnvalue (`Actor.K2_GetActorLocation` (`self.Tank`)))
  (if (`self.CheckForBombPlacement`)
    (bind _returnvalue_2 (`|SpawnActorFromClass` "/Game/TankGame/Blueprints/Weapon/BP_Bomb.BP_Bomb_C" (`KismetMathLibrary.MakeTransform` _returnvalue) "Undefined" "OverrideRootScale" (`self.Tank`) null))
    (`GameplayStatics.PlaySoundAtLocation` "/Game/TankGame/Music/BombPaste.BombPaste" (`Actor.K2_GetActorLocation` _returnvalue_2) (struct) 1.0 1.0 0.0 null null null)
    (`/Engine/EditorBlueprintResources/StandardMacros.IsValid` _returnvalue_2
      (:`Is Valid`
        (add `/Game/TankGame/Blueprints/Weapon/BP_Bomb.BombDestroyed_0` _returnvalue_2 (`|CreateDelegate` :!event `ChangeBombCount`))
        (`/Engine/EditorBlueprintResources/StandardMacros.IncrementInt` (`self.BombCounter`)
          (:`  `
            (return true _returnvalue))))
      (:`Is Not Valid`
        (return false (0.0 0.0 0.0))))
    (else
      (return false (0.0 0.0 0.0)))))

(fn `RicochetTraces`
  (returns (TankFound :type Boolean) (PreviousHit :type "HitResult Structure") (TankToHit :type "/Game/TankGame/Blueprints/Core/BP_Tank Object Reference"))
  (locals (L_TankFound :type Boolean))
  (bind (_previoushit_bblockinghit _previoushit_binitialoverlap _previoushit_time _previoushit_distance _previoushit_location _previoushit_impactpoint _previoushit_normal _previoushit_impactnormal _previoushit_physmat _previoushit_hitactor) (`GameplayStatics.BreakHitResult` (`self.PreviousHit`)))
  (bind (_bblockinghit _binitialoverlap _time _distance _location _impactpoint _normal _impactnormal _physmat _hitactor) (`GameplayStatics.BreakHitResult` (`self.PreviousHit`)))
  (bind (_bblockinghit_2 _binitialoverlap_2 _time_2 _distance_2 _location_2 _impactpoint_2 _normal_2 _impactnormal_2 _physmat_2 _hitactor_2 _hitcomponent _hitbonename _hititem _elementindex _faceindex _tracestart _traceend) (`GameplayStatics.BreakHitResult` (`self.PreviousHit`)))
  (bind _returnvalue (`KismetMathLibrary.MirrorVectorByNormal` (- _traceend _tracestart) _impactnormal_2))
  (bind _returnvalue_2 (+ _impactpoint_2 _returnvalue))
  (if (>= (`self.Number Of Ricochets`) 1)
    (for _ (range 1 (+ (`self.Number Of Ricochets`) 1))
      (bind (_outhit _returnvalue_3) (`KismetSystemLibrary.SphereTraceSingle` (+ _impactpoint_2 (`KismetMathLibrary.Normal` _returnvalue)) _returnvalue_2 2.0 "TraceTypeQuery1" false (`|MakeArray` _previoushit_hitactor) "None" true (struct :`R` 1.0 :`B` 0.840783 :`A` 1.0) (struct :`R` 1.0 :`G` 0.804968 :`A` 1.0) 2.0))
      (set `self.PreviousHit` _outhit)
      (if _returnvalue_3
        (set `self.RicochetEnd` _location)
        (else
          (set `self.RicochetEnd` _returnvalue_2)))
      (bind _asbp_tank (cast `/Game/TankGame/Blueprints/Core/BP_Tank` _hitactor))
      (set `self.TankToHit` _asbp_tank)
      (set `local.L_TankFound` true)
      (break))
    (if (`local.L_TankFound`)
      (return (`local.L_TankFound`) (`self.PreviousHit`) (`self.TankToHit`))
      (else
        (return (`local.L_TankFound`) (`self.PreviousHit`) null)))))

(fn `SetTankSpecification`
  (bind (_datatable _rowname) (break `DataTableRowHandle` (`.Description_2_838EBF994D755D2F64E9E5BCF961BF3C` (break `/Game/TankGame/Blueprints/Core/ST_TankSpecification` (`/Game/TankGame/Blueprints/Core/BP_Tank.Specification` (`self.Tank`))))))
  (bind _returnvalue (`|GetDataTableRow` _datatable _rowname)
    (:`then`
      (bind (_tanktype _canmove _canplacebombs _numberofricochets _numberofbullets _numberofbombs _tankspeed _bullettype _material _color _shootdelta) (break `/Game/TankGame/Blueprints/Core/S_Tank` _returnvalue))
      (set `self.Tank Type` _tanktype)
      (set `self.Can Move` _canmove)
      (set `self.Can Place Bombs` _canplacebombs)
      (set `self.Number Of Ricochets` _numberofricochets)
      (set `self.NumberOfBombs` _numberofbombs)
      (set `self.Bullet Type` _bullettype)
      (set `self.Shoot Delta` _shootdelta)
      (set `self.TankColor` _color)
      (if (`|EnumEquality` (`self.CurGame Mode`) "NewEnumerator2")
        (cast `/Game/TankGame/Blueprints/Player/BP_Player` (`self.Tank`)
          (:`then`
            (set `self.NumberOfBullets` (`/Game/TankGame/Blueprints/Core/GM_Tanks.GetBulletsRemain` (`self.GameMode`))))
          (:`CastFailed`
            (set `self.NumberOfBullets` _numberofbullets :!label _label)))
        (else
          (goto _label))))))

(fn `Shoot`
  (`self.SpawnBullet`))

(fn `SpawnBullet`
  (returns (BulletSpawned :type Boolean))
  (bind _tank (`self.Tank`))
  (bind (_returnvalue_location _returnvalue_rotation _returnvalue_scale) (`KismetMathLibrary.BreakTransform` (`SceneComponent.K2_GetComponentToWorld` (`/Game/TankGame/Blueprints/Core/BP_Tank.Arrow1` (`self.Tank`)))))
  (if (< (`self.BulletCounter`) (`self.NumberOfBullets`))
    (bind _returnvalue (`|SpawnActorFromClass` (`self.Bullet Type`) (`KismetMathLibrary.MakeTransform` _returnvalue_location _returnvalue_rotation _returnvalue_scale) "AlwaysSpawn" "OverrideRootScale" _tank _tank))
    (`/Engine/EditorBlueprintResources/StandardMacros.IsValid` _returnvalue
      (:`Is Valid`
        (bind _output_get (set `self.Bullet` _returnvalue))
        (`GameplayStatics.PlaySoundAtLocation` "/Game/TankGame/Music/Shot.Shot" (`Actor.K2_GetActorLocation` _output_get) (struct) 1.0 1.0 0.0 null null _output_get)
        (if (`|EnumEquality` (`self.CurGame Mode`) "NewEnumerator2")
          (cast `/Game/TankGame/Blueprints/Player/BP_Player` (`self.Tank`)
            (:`then`
              (`/Game/TankGame/Blueprints/Core/GM_Tanks.AddBullets` (`self.GameMode`))
              (`/Engine/EditorBlueprintResources/StandardMacros.DecrementInt` (`self.NumberOfBullets`)
                (:`  `
                  (return true))))
            (:`CastFailed`
              _)))
        (add `/Game/TankGame/Blueprints/Weapon/BP_BulletDefault.BulletDestroyed` (`self.Bullet`) (`|CreateDelegate` :!event `ChangeBulletCount`))
        (`/Engine/EditorBlueprintResources/StandardMacros.IncrementInt` (`self.BulletCounter`)
          (:`  `
            (return true)))))
    (else
      (return false))))